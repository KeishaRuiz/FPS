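; Target actor that counts down a shared target total on overlap and triggers the win screen.
; Each overlap, with no filter on the other actor, decrements TargetHit on FPSGamemode.
; When the counter reaches exactly zero, it creates a win menu widget and adds it to the viewport.
; The target neither destroys nor disables itself, so repeated overlaps keep decrementing the count.
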(event Collision|EventActorBeginOverlap
  (params (OtherActor :type Actor%20Object%20Reference))
  (bind _asfpsgamemode (Utilities|Casting|CastToFPSGamemode (Game|GetGameMode)))
  (bind _result (Math|Integer|DecrementInt (Variables|/Game/FPSGamemode.FPSGamemode_C|GetTargetHit _asfpsgamemode))
    (:%20%20
      (Variables|/Game/FPSGamemode.FPSGamemode_C|SetTargetHit _asfpsgamemode _result)
      (bind _asfpsgamemode_2 (Utilities|Casting|CastToFPSGamemode (Game|GetGameMode)))
      (if (== (Variables|/Game/FPSGamemode.FPSGamemode_C|GetTargetHit _asfpsgamemode_2) 0)
        (bind _returnvalue (UserInterface|CreateWidget "/Game/WinMenu.WinMenu_C"))
        (UserInterface|Viewport|AddtoViewport _returnvalue 0)))))

(fn ConstructionScript)