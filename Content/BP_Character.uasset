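; BP_Character is the playable character, with yaw-relative movement, mouse look, jumping and ammo-limited shooting.
; Left click spends one Ammo to spawn a Projectile_BP at the SpawnProjectile component, or prints a warning when empty.
; BeginPlay adds health and ammo widgets to the viewport.
; Tick polls the player character's Health and, once depleted, destroys it, shows GameOverWidget and disables mouse-over events.
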(event EventBeginPlay
  (bind _returnvalue (UserInterface|CreateWidget "/Game/HealthTrack_BP.HealthTrack_BP_C"))
  (bind _returnvalue_2 (UserInterface|CreateWidget "/Game/AmmoWidget.AmmoWidget_C"))
  (UserInterface|Viewport|AddtoViewport _returnvalue 0))

(event EventTick
  (params (DeltaSeconds :type Float%20%28single-precision%29))
  (bind _asbp_character (Utilities|Casting|CastToBP_Character (Game|GetPlayerCharacter 0)))
  (if (<= (Variables|BP_Character_C|GetHealth _asbp_character) 0.0)
    (Utilities|FlowControl|DoOnce false
      (:Completed
        (Actor|DestroyActor _asbp_character)
        (bind _returnvalue (UserInterface|CreateWidget "/Game/GameOverWidget.GameOverWidget_C"))
        (UserInterface|Viewport|AddtoViewport _returnvalue 0)
        (Variables|/Script/Engine.PlayerController|SetbEnableMouseOverEvents (Game|GetPlayerController 0) false)))))

(event Input|ActionEvents|InputActionJump
  (params (Key :type Key%20Structure :default "None"))
  (:Pressed
    (Character|Jump)))

(event Input|AxisEvents|InputAxisFoward/Backward
  (params (AxisValue :type Float%20%28single-precision%29))
  (Pawn|Input|AddMovementInput (Math|Vector|GetForwardVector (Math|Rotator|MakeRotator 0.0 0.0 (.Yaw (Math|Rotator|BreakRotator (Pawn|GetControlRotation :!class /Script/Engine.Pawn))))) AxisValue false))

(event Input|AxisEvents|InputAxisRight/Left
  (params (AxisValue :type Float%20%28single-precision%29))
  (Pawn|Input|AddMovementInput (Math|Vector|GetRightVector (Math|Rotator|MakeRotator 0.0 0.0 (.Yaw (Math|Rotator|BreakRotator (Pawn|GetControlRotation :!class /Script/Engine.Pawn))))) AxisValue false))

(event Input|AxisEvents|InputAxisTurn
  (params (AxisValue :type Float%20%28single-precision%29))
  (Pawn|Input|AddControllerYawInput AxisValue))

(event Input|AxisEvents|InputAxisLookUp/Down
  (params (AxisValue :type Float%20%28single-precision%29))
  (Pawn|Input|AddControllerPitchInput AxisValue))

(event Input|MouseEvents|LeftMouseButton
  (params (Key :type Key%20Structure :default "None"))
  (:Pressed
    (if (> (Variables|Default|GetAmmo) 0)
      (Variables|Default|SetAmmo (- (Variables|Default|GetAmmo) 1))
      (Game|SpawnActorfromClass "/Game/Projectile_BP.Projectile_BP_C" (Transformation|GetWorldTransform (Variables|Default|GetSpawn_projectile)) "Undefined" 0 0)
      (else
        (Development|PrintString "No ammo left!")))))

(fn ConstructionScript)